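; WP_Shrike is a NeoTerra actor that trails particles and reorients itself when it overlaps a wall.
; Each Tick feeds the particle system a ParticleVelocity vector pointing backward along the actor's forward axis, with slight random cone jitter.
; On overlap with a "Wall"-tagged actor, StickToWall only sets rotation, using that actor's rotated up vector as a placeholder surface normal, noted as likely non-working.
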(event Collision|EventActorBeginOverlap
  (params (OtherActor :type Actor%20Object%20Reference))
  (CallFunction|SticktoWall OtherActor))

(event EventTick
  (params (DeltaSeconds :type Float%20%28single-precision%29))
  (CallFunction|SetParticleVelocity))

(fn ConstructionScript)

(fn SetParticleVelocity
  (bind _returnvalue (Transformation|GetActorForwardVector))
  (Effects|Components|ParticleSystem|SetVectorParameter (Variables|Default|GetParticleSystem) "ParticleVelocity" (+ (* _returnvalue -2e+02) (* (Class|KismetMathLibrary|RandomUnitVectorinCone _returnvalue 0.2) -3e+01))))

(fn SticktoWall
  (params (OtherActor :type Actor%20Object%20Reference%20%28by%20ref%29))
  (if (Actor|ActorHasTag OtherActor "Wall")
    (Transformation|SetActorRotation (Math|Conversions|RotationFromXVector (Math|Vector|RotateVector (Transformation|GetActorUpVector OtherActor) (Transformation|GetActorRotation))))))